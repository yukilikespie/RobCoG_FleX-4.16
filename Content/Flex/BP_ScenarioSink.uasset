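; Sink scenario actor, apparently for a Flex fluid demo, that turns the tap's particle emitter on and off as the tap top rotates.
; BeginPlay enables player 0 input.
; Each Tick compares the world yaw of TapTopToTapMiddle with TapTopTwist, activating PSTapEmitter at or above it and deactivating it below.
; A debug print and logic to move the emitter with the tap bottom are left disconnected.
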(event `self.ReceiveBeginPlay`
  ;[1 1 1] Enable Input
  (`self.EnableInput` (`GameplayStatics.GetPlayerController` 0)))

(event `self.ReceiveTick`
  (params (DeltaSeconds :type "Float (single-precision)"))
  (bind _ps_tapemitter (`self.PS_TapEmitter`))
  ;[1 1 1] Activate/Deactivate PS Tap Emitter TapTop rotation changes
  (`/Engine/EditorBlueprintResources/StandardMacros.CompareFloat` (.yaw (`SceneComponent.K2_GetComponentRotation` (`self.TapTopToTapMiddle`))) (`self.TapTopTwist`)
    (:`>`
      (`ActorComponent.Activate` _ps_tapemitter false :!label _label))
    (:`==`
      (goto _label))
    (:`<`
      (if (`ActorComponent.IsActive` (`self.PS_TapEmitter`))
        (`ActorComponent.Deactivate` _ps_tapemitter)))))

(fn `UserConstructionScript`)