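; BP_ScenarioSink is a sink actor with a tap particle emitter that the player switches on and off from the keyboard.
; BeginPlay enables input for player 0, E toggles PSTapEmitter, and H sets TapBottom's relative rotation to zero.
; The TapBottom overlap handler does nothing, and the logic to move the fluid emitter with TapBottom is disconnected.
; Debug strings print on BeginPlay and on each E press.
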(event `self.ReceiveBeginPlay`
  ;[1 1 1] Enable Input
  (`self.EnableInput` (`GameplayStatics.GetPlayerController` 0))
  (`KismetSystemLibrary.PrintString` "Input Enabled"))

(event `Key|E`
  (params (Key :type "Key Structure" :default "AnyKey"))
  (bind _ps_tapemitter (`self.PS_TapEmitter`))
  ;[1 1 1] Activate/Deactivate PS Tap Emitter when "E" key is pressed
  (:`Pressed`
    (`KismetSystemLibrary.PrintString` "Hello")
    (if (`ActorComponent.IsActive` (`self.PS_TapEmitter`))
      (`ActorComponent.Deactivate` _ps_tapemitter)
      (else
        (`ActorComponent.Activate` _ps_tapemitter false)))))

(event `Key|H`
  (params (Key :type "Key Structure" :default "AnyKey"))
  (:`Pressed`
    (`SceneComponent.K2_SetRelativeRotation` :`self` (`self.TapBottom`) :`bSweep` true :`bTeleport` true)))

(event `self.TapBottom.OnComponentBeginOverlap`
  (params (OverlappedComponent :type "PrimitiveComponent Object Reference") (OtherActor :type "Actor Object Reference") (OtherComp :type "PrimitiveComponent Object Reference") (OtherBodyIndex :type Integer) (bFromSweep :type Boolean) (SweepResult :type "HitResult Structure (by ref)"))
  (if true
    _))

(fn `UserConstructionScript`)