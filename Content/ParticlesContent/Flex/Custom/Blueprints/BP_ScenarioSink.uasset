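; BP_ScenarioSink is a sink scenario actor that simulates running tap water with a Flex particle emitter.
; While the scenario is active, one input toggles the tap emitter and another moves a plug box up or down to start or stop the water flow.
; A separate kill input fires a particle event to clear the water regardless of active state.
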(event `InputAction|Interact2`
  (params (Key :type "Key Structure" :default "AnyKey"))
  (bind _box (`self.Box`))
  ;[1 1 1] Moving the plug to start/stop the waterflow
  (:`Pressed`
    (if (`self.isActive`)
      (bind _output_get (set `self.PlugActive` (not (`self.PlugActive`))))
      (if _output_get
        (`KismetSystemLibrary.MoveComponentTo` _box (-2.0 -15.0 -28.0))
        (else
          (`KismetSystemLibrary.MoveComponentTo` _box (-2.0 -15.0 -35.0)))))))

(event `/Game/ParticlesContent/Flex/Custom/Blueprints/BPI_Scenario.ToggleActive`
  (set `self.isActive` (not (`self.isActive`))))

(event `InputAction|Interact1`
  (params (Key :type "Key Structure" :default "AnyKey"))
  (:`Pressed`
    (if (`self.isActive`)
      (`ActorComponent.ToggleActive` (`self.PS_TapEmitter`)))))

(event `InputAction|KillParticles`
  (params (Key :type "Key Structure" :default "AnyKey"))
  (:`Pressed`
    (`ParticleSystemComponent.GenerateParticleEvent` (`self.PS_TapEmitter`) "FlexWaterEmitterKillEvent" 0.0 (0.0 0.0 0.0) (0.0 0.0 0.0) (0.0 0.0 0.0))))

(fn `UserConstructionScript`)